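; Player character that measures SpatialOS network latency by chaining latency payloads and worker-tagged trace events through RPCs and replicated properties.
; The autonomous client loops staggered timers for server-to-client RPC, multicast and property-update traces, with debug keys for manual runs and an interaction trace.
; While authoritative under spatial networking, it also traces cross-server RPC and property round trips to nearby non-authoritative characters, reserving targets through LatencyGameMode.
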(event Custom|OnInput_InteractionClientComplete
  (params (SpatialPayload :type Spatial%20Latency%20Payload%20Structure))
  (bind _returnvalue (Class|SpatialLatencyTracer|EndLatencyTrace SpatialPayload))
  (if _returnvalue
    (Development|PrintString "Client Interaction Complete")
    (else
      (Development|PrintString "Client Interaction Failed"))))

(event Custom|OnInput_MulticastRPC
  (params (SpatialPayload :type Spatial%20Latency%20Payload%20Structure))
  (Networking|SwitchHasAuthority
    (:Remote
      (bind _returnvalue (Class|SpatialLatencyTracer|EndLatencyTrace SpatialPayload))
      (if _returnvalue
        (Development|PrintString "Multicast RPC Trace Complete")
        (bind _outuserspanid (Class|SpatialEventTracerUserInterface|GetActiveSpanId))
        (CallFunction|TraceEventBasicwithWorkerID "latency.multicast_end" (Utilities|Array|MakeArray _outuserspanid))
        (else
          (Development|PrintString "Failed to end Multicast RPC Trace"))))))

(event Custom|BeginCrossServerPropertyUpdateTrace
  (Networking|SwitchHasAuthority
    (:Authority
      (bind _targetplayer (CallFunction|FindTargetinOtherZone 1))
      (Utilities|IsValid _targetplayer
        (:Is%20Valid
          (CallFunction|AddinUsePropertyUpdateTarget _targetplayer)
          (bind (_outlatencypayload _returnvalue) (Class|SpatialLatencyTracer|BeginLatencyTrace "Input > Cross Server > RPC to Property Update"))
          (if _returnvalue
            (bind (_outcontinuedlatencypayload _returnvalue_2) (Class|SpatialLatencyTracer|ContinueLatencyTraceRPC _targetplayer "OnInput_CrossServerPropertyUpdate" "Input > Cross Server > RPC to Property Update" _outlatencypayload))
            (if _returnvalue_2
              (bind _return_value (CallFunction|TraceEventBasicwithWorkerID "latency.cross_server_property" (Utilities|Array|MakeArray "")))
              (Class|SpatialEventTracerUserInterface|TraceRPC (delegate Custom|CustomEvent) _return_value))))))))

(event Custom|OnInput_ServerRPC
  (params (UseMulticast :type Boolean) (SpatialPayload :type Spatial%20Latency%20Payload%20Structure))
  (if UseMulticast
    (bind (_outcontinuedlatencypayload _returnvalue) (Class|SpatialLatencyTracer|ContinueLatencyTraceRPC self "OnInput_MulticastRPC" "ServerAck > Multicast RPC" SpatialPayload))
    (if _returnvalue
      (bind _outuserspanid (Class|SpatialEventTracerUserInterface|GetActiveSpanId))
      (bind _return_value (CallFunction|TraceEventBasicwithWorkerID "latency.multicast_rpc" (Utilities|Array|MakeArray _outuserspanid)))
      (Class|SpatialEventTracerUserInterface|TraceRPC (delegate Custom|Server%20Multicast%20RPC) _return_value)
      (else
        (Development|PrintString "Failed to continue Multicast RPC Trace")))
    (else
      (bind (_outcontinuedlatencypayload_2 _returnvalue_2) (Class|SpatialLatencyTracer|ContinueLatencyTraceRPC self "OnInput_ClientRPC" "ServerAck > Client RPC" SpatialPayload))
      (if _returnvalue_2
        (bind _outuserspanid_2 (Class|SpatialEventTracerUserInterface|GetActiveSpanId))
        (bind _return_value_2 (CallFunction|TraceEventBasicwithWorkerID "latency.client_rpc" (Utilities|Array|MakeArray _outuserspanid_2)))
        (Class|SpatialEventTracerUserInterface|TraceRPC (delegate Custom|Server%20Client%20RPC) _return_value_2)
        (else
          (Development|PrintString "Failed to continue Client Trace"))))))

(event Custom|OnInput_CrossServerPropertyUpdate
  (params (LatencyPayload :type Spatial%20Latency%20Payload%20Structure))
  (bind _self self)
  (bind (_outcontinuedlatencypayload _returnvalue) (Class|SpatialLatencyTracer|ContinueLatencyTraceProperty _self "CrossServerProperty" "Input > Cross Server > RPC to Property Update" LatencyPayload))
  (if _returnvalue
    (bind _return_value (CallFunction|TraceEventBasicwithWorkerID "latency.cross_server_property_update" (Utilities|Array|MakeArray "")))
    (Class|SpatialEventTracerUserInterface|TraceProperty self _return_value)
    (Variables|Default|SetCrossServerProperty _outcontinuedlatencypayload)
    (CallFunction|RemoveinUsePropertyUpdateTarget _self)))

(event Custom|OnInput_TriggerInteractable
  (params (Payload :type Spatial%20Latency%20Payload%20Structure))
  (bind _returnvalue (Class|SpatialLatencyTracer|ContinueLatencyTraceTagged self "InteractableStarted" "Input > Server RPC > Interaction" Payload))
  (if _returnvalue
    (Utilities|FlowControl|Delay 0.5)
    (bind _returnvalue_2 (Class|SpatialLatencyTracer|RetrievePayload self "InteractableStarted"))
    (bind (_outcontinuedlatencypayload _returnvalue_3) (Class|SpatialLatencyTracer|ContinueLatencyTraceRPC self "OnInput_InteractionClientComplete" "Input > Server RPC > Interaction" _returnvalue_2))
    (if _returnvalue_3
      (CallFunction|OnInputInteractionClientComplete _outcontinuedlatencypayload)
      (else
        (Development|PrintString "Failed to continue inteaction on server")))
    (else
      (Development|PrintString "Failed to continue interaction trace"))))

(event Custom|OnSetRunId
  (params (TraceMetadata :type String))
  (CallFunction|SetRunId TraceMetadata))

(event Custom|RPC%20Trace%20Delegate
  (CallFunction|OnInputServerRPC false (stale Custom|BeginClientRPCTrace _outcontinuedlatencypayload)))

(event Custom|CrossServerRPC
  (CallFunction|OnInputCrossServerCall (stale Custom|BeginCrossServerRPCTrace _targetplayer) self (stale Custom|BeginCrossServerRPCTrace _outcontinuedlatencypayload)))

(event Custom|CrossServerReply
  (CallFunction|OnInputCrossServerReply (stale Custom|OnInput_CrossServerCall SourcePlayer) (stale Custom|OnInput_CrossServerCall _outcontinuedlatencypayload))
  (CallFunction|RemoveinUseRPCTarget self))

(event Custom|Server%20Client%20RPC
  (CallFunction|OnInputClientRPC (stale Custom|OnInput_ServerRPC _outcontinuedlatencypayload_2)))

(event Custom|RPC%20Trace%20Property%20Update
  (CallFunction|OnInputPropertyUpdate (stale Custom|BeginPropertyUpdate _outcontinuedlatencypayload)))

(event Custom|OnInput_ClientRPC
  (params (SpatialPayload :type Spatial%20Latency%20Payload%20Structure))
  (bind _returnvalue (Class|SpatialLatencyTracer|EndLatencyTrace SpatialPayload))
  (if _returnvalue
    (Development|PrintString "Client RPC Trace Complete")
    (bind _outuserspanid (Class|SpatialEventTracerUserInterface|GetActiveSpanId))
    (CallFunction|TraceEventBasicwithWorkerID "latency.client_end" (Utilities|Array|MakeArray _outuserspanid))
    (else
      (Development|PrintString "Failed to end Client RPC Trace"))))

(event Custom|Server%20Multicast%20RPC
  (CallFunction|OnInputMulticastRPC (stale Custom|OnInput_ServerRPC _outcontinuedlatencypayload)))

(event Custom|RPC%20Trace%20Delegate%20Multicast
  (CallFunction|OnInputServerRPC true (stale Custom|BeginMulticastRPC _outcontinuedlatencypayload)))

(event Custom|CustomEvent
  (CallFunction|OnInputCrossServerPropertyUpdate (stale Custom|BeginCrossServerPropertyUpdateTrace _targetplayer) (stale Custom|BeginCrossServerPropertyUpdateTrace _outcontinuedlatencypayload)))

(event Custom|BeginClientRPCTrace
  (bind (_outlatencypayload _returnvalue) (Class|SpatialLatencyTracer|BeginLatencyTrace "Input > Server RPC > Client RPC"))
  (if _returnvalue
    (bind (_outcontinuedlatencypayload _returnvalue_2) (Class|SpatialLatencyTracer|ContinueLatencyTraceRPC self "OnInput_ServerRPC" "Input > Server RPC > Client RPC" _outlatencypayload))
    (if _returnvalue_2
      (bind _return_value (CallFunction|TraceEventBasicwithWorkerID "latency.server_rpc" (Utilities|Array|MakeArray "")))
      (Class|SpatialEventTracerUserInterface|TraceRPC (delegate Custom|RPC%20Trace%20Delegate) _return_value)
      (else
        (Development|PrintString "Failed to start Client RPC Trace" :!label _label)))
    (else
      (goto _label))))

(event Custom|BeginMulticastRPC
  (bind (_outlatencypayload _returnvalue) (Class|SpatialLatencyTracer|BeginLatencyTrace "Input > Server RPC > Multicast RPC"))
  (if _returnvalue
    (bind _outcontinuedlatencypayload (Class|SpatialLatencyTracer|ContinueLatencyTraceRPC self "OnInput_ServerRPC" "Input > Server RPC > Multicast RPC" _outlatencypayload))
    (if true
      (bind _return_value (CallFunction|TraceEventBasicwithWorkerID "latency.server_rpc" (Utilities|Array|MakeArray "")))
      (Class|SpatialEventTracerUserInterface|TraceRPC (delegate Custom|RPC%20Trace%20Delegate%20Multicast) _return_value)
      (else
        (Development|PrintString "Failed to start Multicast RPC Trace" :!label _label)))
    (else
      (goto _label))))

(event Custom|BeginPropertyUpdate
  (bind (_outlatencypayload _returnvalue) (Class|SpatialLatencyTracer|BeginLatencyTrace "Input > Server RPC > Property Update"))
  (if _returnvalue
    (bind (_outcontinuedlatencypayload _returnvalue_2) (Class|SpatialLatencyTracer|ContinueLatencyTraceRPC self "OnInput_PropertyUpdate" "Input > Server RPC > Property Update" _outlatencypayload))
    (if _returnvalue_2
      (bind _return_value (CallFunction|TraceEventBasicwithWorkerID "latency.server_rpc" (Utilities|Array|MakeArray "")))
      (Class|SpatialEventTracerUserInterface|TraceRPC (delegate Custom|RPC%20Trace%20Property%20Update) _return_value)
      (else
        (Development|PrintString "Failed to start property update" :!label _label)))
    (else
      (goto _label))))

(event Custom|BeginCrossServerRPCTrace
  (Networking|SwitchHasAuthority
    (:Authority
      (bind _targetplayer (CallFunction|FindTargetinOtherZone))
      (Utilities|IsValid _targetplayer
        (:Is%20Valid
          (CallFunction|AddinUseRPCTarget _targetplayer)
          (bind (_outlatencypayload _returnvalue) (Class|SpatialLatencyTracer|BeginLatencyTrace "Input > Cross Server > RPC to RPC"))
          (if _returnvalue
            (bind (_outcontinuedlatencypayload _returnvalue_2) (Class|SpatialLatencyTracer|ContinueLatencyTraceRPC _targetplayer "OnInput_CrossServerCall" "Input > Cross Server > RPC to RPC" _outlatencypayload))
            (if _returnvalue_2
              (bind _return_value (CallFunction|TraceEventBasicwithWorkerID "latency.cross_server_rpc" (Utilities|Array|MakeArray "")))
              (Class|SpatialEventTracerUserInterface|TraceRPC (delegate Custom|CrossServerRPC) _return_value))))))))

(event Custom|OnInput_CrossServerCall
  (params (SourcePlayer :type Latency%20Player%20Character%20BP%20Object%20Reference) (LatencyPayload :type Spatial%20Latency%20Payload%20Structure))
  (bind (_outcontinuedlatencypayload _returnvalue) (Class|SpatialLatencyTracer|ContinueLatencyTraceRPC SourcePlayer "OnInput_CrossServerReply" "Input > Cross Server > RPC to RPC" LatencyPayload))
  (if _returnvalue
    (if (Ability|HasAuthority SourcePlayer)
      (Development|PrintString (Utilities|String|Append "Source Player ( " (Class|SpatialStatics|GetActorEntityIdasString SourcePlayer) " ) is locally authoritative, aborting cross server trace."))
      (else
        (bind _outuserspanid (Class|SpatialEventTracerUserInterface|GetActiveSpanId))
        (bind _return_value (CallFunction|TraceEventBasicwithWorkerID "latency.cross_server_reply" (Utilities|Array|MakeArray _outuserspanid)))
        (Class|SpatialEventTracerUserInterface|TraceRPC (delegate Custom|CrossServerReply) _return_value)))))

(event Custom|OnInput_CrossServerReply
  (params (LatencyPayload :type Spatial%20Latency%20Payload%20Structure))
  (Class|SpatialLatencyTracer|EndLatencyTrace LatencyPayload)
  (bind _outuserspanid (Class|SpatialEventTracerUserInterface|GetActiveSpanId))
  (CallFunction|TraceEventBasicwithWorkerID "latency.cross_server_end" (Utilities|Array|MakeArray _outuserspanid)))

(event Custom|OnInput_PropertyUpdate
  (params (SpatialPayload :type Spatial%20Latency%20Payload%20Structure))
  (bind _outcontinuedlatencypayload (Class|SpatialLatencyTracer|ContinueLatencyTraceProperty self "ServerProperty" "Input > Server RPC > Property Update" SpatialPayload))
  (if true
    (bind _outuserspanid (Class|SpatialEventTracerUserInterface|GetActiveSpanId))
    (bind _return_value (CallFunction|TraceEventBasicwithWorkerID "latency.property_update" (Utilities|Array|MakeArray _outuserspanid)))
    (Class|SpatialEventTracerUserInterface|TraceProperty self _return_value)
    (Variables|Default|SetServerProperty _outcontinuedlatencypayload)
    (else
      (Development|PrintString "Failed to continue property update"))))

(event EventBeginPlay
  (if (Networking|IsServer)
    _
    (else
      (CallFunction|OnSetRunId (Class|SpatialLatencyTracer|GetTraceMetadata))))
  ;[1 1 1] Delay required because role can be incorrect in spatial on startup :(
  (Utilities|FlowControl|Delay 0.2)
  (if (Utilities|Enum|Equal(Enum) (Networking|GetLocalRole) "ROLE_AutonomousProxy")
    (Utilities|Time|SetTimerbyEvent (delegate Custom|BeginClientRPCTrace) 5.0 true)
    (Utilities|FlowControl|Delay 1.0)
    (Utilities|Time|SetTimerbyEvent (delegate Custom|BeginMulticastRPC) 5.0 true)
    (Utilities|FlowControl|Delay 1.0)
    (Utilities|Time|SetTimerbyEvent (delegate Custom|BeginPropertyUpdate) 5.0 true)))

(event Collision|EventActorBeginOverlap
  (params (OtherActor :type Actor%20Object%20Reference)))

(event EventTick
  (params (DeltaSeconds :type Float%20%28single-precision%29)))

(event EventAuthorityGained
  (if (Class|SpatialStatics|IsSpatialNetworkingEnabled)
    (bind _returnvalue (Utilities|Time|SetTimerbyEvent (delegate Custom|BeginCrossServerRPCTrace) 5.0 true))
    (Variables|Default|SetCrossServerRPCTimer _returnvalue)
    (Utilities|FlowControl|Delay 1.0)
    (bind _returnvalue_2 (Utilities|Time|SetTimerbyEvent (delegate Custom|BeginCrossServerPropertyUpdateTrace) 5.0 true))
    (Variables|Default|SetCrossServerPropertyTimer _returnvalue_2)))

(event EventAuthorityLost
  (Utilities|Time|ClearandInvalidateTimerbyHandle (Variables|Default|GetCrossServerRPCTimer))
  (Utilities|Time|ClearandInvalidateTimerbyHandle (Variables|Default|GetCrossServerPropertyTimer)))

(event Input|KeyboardEvents|I
  (params (Key :type Key%20Structure :default "None"))
  (:Released
    (bind (_outlatencypayload _returnvalue) (Class|SpatialLatencyTracer|BeginLatencyTrace "Input > Server RPC > Client RPC"))
    (if _returnvalue
      (bind (_outcontinuedlatencypayload _returnvalue_2) (Class|SpatialLatencyTracer|ContinueLatencyTraceRPC self "OnInput_ServerRPC" "Input > Server RPC > Client RPC" _outlatencypayload))
      (if _returnvalue_2
        (bind _return_value (CallFunction|TraceEventBasicwithWorkerID "latency.server_rpc" (Utilities|Array|MakeArray "")))
        (Class|SpatialEventTracerUserInterface|TraceRPC (delegate Custom|RPC%20Trace%20Delegate) _return_value)
        (else
          (Development|PrintString "Failed to start Client RPC Trace" :!label _label)))
      (else
        (goto _label)))))

(event Input|KeyboardEvents|N
  (params (Key :type Key%20Structure :default "None"))
  (:Released
    (bind (_outlatencypayload _returnvalue) (Class|SpatialLatencyTracer|BeginLatencyTrace "Input > Server RPC > Interactable"))
    (if _returnvalue
      (bind (_outcontinuedlatencypayload _returnvalue_2) (Class|SpatialLatencyTracer|ContinueLatencyTraceRPC self "OnInput_TriggerInteractable" "Input > Server RPC > Interactable" _outlatencypayload))
      (if _returnvalue_2
        (CallFunction|OnInputTriggerInteractable _outcontinuedlatencypayload)
        (else
          (Development|PrintString "Failed to start interactable" :!label _label)))
      (else
        (goto _label)))))

(event Input|KeyboardEvents|K
  (params (Key :type Key%20Structure :default "None"))
  (:Released
    (bind (_outlatencypayload _returnvalue) (Class|SpatialLatencyTracer|BeginLatencyTrace "Input > Server RPC > Multicast RPC"))
    (if _returnvalue
      (bind _outcontinuedlatencypayload (Class|SpatialLatencyTracer|ContinueLatencyTraceRPC self "OnInput_ServerRPC" "Input > Server RPC > Multicast RPC" _outlatencypayload))
      (if true
        (bind _return_value (CallFunction|TraceEventBasicwithWorkerID "latency.server_rpc" (Utilities|Array|MakeArray "")))
        (Class|SpatialEventTracerUserInterface|TraceRPC (delegate Custom|RPC%20Trace%20Delegate%20Multicast) _return_value)
        (else
          (Development|PrintString "Failed to start Multicast RPC Trace" :!label _label)))
      (else
        (goto _label)))))

(event Input|KeyboardEvents|J
  (params (Key :type Key%20Structure :default "None"))
  (:Released
    (Class|SpatialLatencyTracer|DebugSendTestTrace)))

(event Input|KeyboardEvents|M
  (params (Key :type Key%20Structure :default "None"))
  (:Released
    (bind (_outlatencypayload _returnvalue) (Class|SpatialLatencyTracer|BeginLatencyTrace "Input > Server RPC > Property Update"))
    (if _returnvalue
      (bind (_outcontinuedlatencypayload _returnvalue_2) (Class|SpatialLatencyTracer|ContinueLatencyTraceRPC self "OnInput_PropertyUpdate" "Input > Server RPC > Property Update" _outlatencypayload))
      (if _returnvalue_2
        (bind _return_value (CallFunction|TraceEventBasicwithWorkerID "latency.server_rpc" (Utilities|Array|MakeArray "")))
        (Class|SpatialEventTracerUserInterface|TraceRPC (delegate Custom|RPC%20Trace%20Property%20Update) _return_value)
        (else
          (Development|PrintString "Failed to start property update" :!label _label)))
      (else
        (goto _label)))))

(fn ConstructionScript
  (Variables|Default|SetWorkerID (Guid|ToString(Guid) (Guid|NewGuid))))

(fn OnRepServerProperty
  (Networking|SwitchHasAuthority
    (:Remote
      (bind _returnvalue (Class|SpatialLatencyTracer|EndLatencyTrace (Variables|Default|GetServerProperty)))
      (bind _outuserspanid (Class|SpatialEventTracerUserInterface|GetActiveSpanId))
      (CallFunction|TraceEventBasicwithWorkerID "latency.property_received" (Utilities|Array|MakeArray _outuserspanid))
      (if _returnvalue
        (Development|PrintString "Successfully finished component update trace")
        (else
          (Development|PrintString "Failed to end property update trace"))))))

(fn FindTargetinOtherZone
  (params (SearchType :type Integer))
  (bind _self self)
  (bind _outactors (Actor|GetAllActorsOfClass "LatencyPlayerCharacter_BP_C"))
  (bind _array_element (Utilities|Array|ForEachLoopwithBreak _outactors :!label _label)
    (:LoopBody
      (if (Math|Boolean|ANDBoolean (not (Ability|HasAuthority _array_element)) (!= _array_element _self) (<= (Transformation|GetDistanceTo _array_element _self) 1.25e+04))
        (bind _aslatency_game_mode (Utilities|Casting|CastToLatencyGameMode (Game|GetGameMode)))
        (switch int SearchType
          (:Default
            (if (not (Utilities|Array|ContainsItem (Variables|/Game/Latency/LatencyGameMode.LatencyGameMode_C|GetRPC_to_PropertyTargets _aslatency_game_mode) _array_element))
              (LocalVariables|SetTarget _array_element :!label _label_2)
              (goto _label Break)))
          (:0
            (if (not (Utilities|Array|ContainsItem (Variables|/Game/Latency/LatencyGameMode.LatencyGameMode_C|GetRPC_to_RPC_Targets _aslatency_game_mode) _array_element))
              (goto _label_2))))))
    (:Completed
      (return (LocalVariables|GetTarget)))))

(fn OnRepCrossServerProperty
  (Networking|SwitchHasAuthority
    (:Remote
      (if (Networking|IsServer)
        (Class|SpatialLatencyTracer|EndLatencyTrace (Variables|Default|GetCrossServerProperty))
        (bind _outuserspanid (Class|SpatialEventTracerUserInterface|GetActiveSpanId))
        (CallFunction|TraceEventBasicwithWorkerID "latency.property_received" (Utilities|Array|MakeArray _outuserspanid))))))

(fn SetRunId
  (params (TraceMetadata :type String))
  (bind _aslatency_game_mode (Utilities|Casting|CastToLatencyGameMode (Game|GetGameMode)))
  (Variables|/Game/Latency/LatencyGameMode.LatencyGameMode_C|SetClientTraceMetadata _aslatency_game_mode TraceMetadata)
  (Development|PrintString (Utilities|String|Append "TraceMetadata: " TraceMetadata)))

(fn AddinUsePropertyUpdateTarget
  (params (PlayerTarget :type Latency%20Player%20Character%20BP%20Object%20Reference))
  (bind _aslatency_game_mode (Utilities|Casting|CastToLatencyGameMode (Game|GetGameMode)))
  (Default|AddinUsePropertyTarget _aslatency_game_mode PlayerTarget))

(fn RemoveinUsePropertyUpdateTarget
  (params (PlayerTarget :type Latency%20Player%20Character%20BP%20Object%20Reference))
  (bind _aslatency_game_mode (Utilities|Casting|CastToLatencyGameMode (Game|GetGameMode)))
  (Default|RemoveinUsePropertyTarget _aslatency_game_mode PlayerTarget))

(fn AddinUseRPCTarget
  (params (TargetPlayer :type Latency%20Player%20Character%20BP%20Object%20Reference))
  (bind _aslatency_game_mode (Utilities|Casting|CastToLatencyGameMode (Game|GetGameMode)))
  (Default|AddinUseRPCTarget _aslatency_game_mode TargetPlayer))

(fn RemoveinUseRPCTarget
  (params (PlayerTarget :type Latency%20Player%20Character%20BP%20Object%20Reference))
  (bind _aslatency_game_mode (Utilities|Casting|CastToLatencyGameMode (Game|GetGameMode)))
  (Default|RemoveinUseRPCTarget _aslatency_game_mode PlayerTarget))

(fn TraceEventBasicwithWorkerID
  (params (Type :type String) (Causes :type Array%20of%20User%20Span%20Id%20Structures))
  (bind _returnvalue (Class|SpatialEventTracerUserInterface|TraceEventwithCauses Type "" (Utilities|Map|MakeMap "worker_id" (Variables|Default|GetWorkerID)) Causes))
  (return _returnvalue))