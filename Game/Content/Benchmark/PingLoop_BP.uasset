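; Benchmark Blueprint that generates a repeating ping load to exercise server and multicast events.
; After a startup delay, if its owner has authority, it starts a server loop that re-invokes itself after random delays.
; Each pass builds an arbitrary random-integer payload, then either multicasts it or calls the server increment directly, depending on the Multicast flag.
; The multicast handler ignores the payload and calls that same server event, which increments the Pings counter.
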(event Custom|Multicast_Ping
  (params (ArbitraryLoad :type Array%20of%20Integers))
  (CallFunction|ServerIncPing))

(event Custom|Server_IncPing
  (Math|Integer|IncrementInt (Variables|Default|GetPings)))

(event Custom|Server_PingLoop
  (bind _array (Utilities|Array|MakeArray 0))
  (for _index (range 0 0)
    (for _index_2 (range 0 5)
      (Utilities|Array|Add _array (Math|Random|RandomInteger 0)))
    (if (Variables|Default|GetMulticast)
      (CallFunction|MulticastPing _array)
      (else
        (CallFunction|ServerIncPing)))
    (Utilities|FlowControl|Delay (Math|Random|RandomFloat))
    (CallFunction|ServerPingLoop)))

(event EventBeginPlay
  (Utilities|FlowControl|Delay 8.0)
  (if (Ability|HasAuthority (Components|GetOwner))
    (CallFunction|ServerPingLoop)))

(event EventTick
  (params (DeltaSeconds :type Float%20%28single-precision%29)))