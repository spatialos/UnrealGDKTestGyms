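; Benchmark actor component that generates continually changing random data, apparently as a replication test load.
; On BeginPlay it waits, then starts the server update only if its owner has authority.
; Each update resets Vector, Transform and Rotator arrays and appends random entries in a short loop.
; A random Delay inside that loop calls the update again, keeping the churn running indefinitely.
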(event Custom|Server_Update
  (bind _returnvalue (Math|Random|RandomUnitVector))
  (bind _output_get (Variables|Default|SetVector (Utilities|Array|MakeArray "0, 0, 0")))
  (bind _output_get_2 (Variables|Default|SetTransform (Utilities|Array|MakeArray "")))
  (bind _output_get_3 (Variables|Default|SetRotator (Utilities|Array|MakeArray "0, 0, 0")))
  (for _index (range 0 4)
    (Utilities|Array|Add _output_get _returnvalue)
    (Utilities|Array|Add _output_get_2 (Math|Conversions|ToTransform(Vector) _returnvalue))
    (Utilities|Array|Add _output_get_3 (Math|Random|RandomRotator false))
    (Utilities|FlowControl|Delay (Math|Random|RandomFloat))
    (CallFunction|ServerUpdate)))

(event EventBeginPlay
  (Utilities|FlowControl|Delay 8.0)
  (if (Ability|HasAuthority (Components|GetOwner))
    (CallFunction|ServerUpdate)))

(event EventTick
  (params (DeltaSeconds :type Float%20%28single-precision%29)))