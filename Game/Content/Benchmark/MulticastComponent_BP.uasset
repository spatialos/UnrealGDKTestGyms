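; Actor component that benchmarks multicast RPC traffic in a network test.
; After a delay from BeginPlay, the server starts a self-repeating ping loop on actors where it has authority.
; Each pass sends a multicast ping, counts server calls and waits a random sub-second delay before repeating, while each receiver of the multicast increments its own receive counter.
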(event Custom|Multicast_Ping
  (Math|Integer|IncrementInt (Variables|Default|GetClientReceives)))

(event Custom|Server_PingLoop
  (CallFunction|MulticastPing)
  (Math|Integer|IncrementInt (Variables|Default|GetServerCalls)
    (:%20%20
      (Utilities|FlowControl|Delay (Math|Random|RandomFloat))
      (CallFunction|ServerPingLoop))))

(event EventBeginPlay
  (Utilities|FlowControl|Delay 8.0)
  (if (Ability|HasAuthority (Components|GetOwner))
    (CallFunction|ServerPingLoop)))

(event EventTick
  (params (DeltaSeconds :type Float%20%28single-precision%29)))