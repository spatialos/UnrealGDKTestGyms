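; Benchmark component that repeatedly spawns and retires a drop cube at its owner's transform, with authority and entity-ID logging.
; The server cube logic loops: with owner authority it spawns a cube, waits a random delay, flags it to self-destruct, then re-runs, polling while the cube remains valid.
; Losing authority or ending play also flags any live cube to self-destruct, so cleanup does not depend on the loop.
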(event Custom|Server_CubeLogic
  (Utilities|IsValid (Variables|Default|GetSpawnedCube)
    (:Is%20Valid
      (Utilities|FlowControl|Delay 1.0)
      (CallFunction|ServerCubeLogic))
    (:Is%20Not%20Valid
      (if (Ability|HasAuthority (Components|GetOwner))
        (bind _returnvalue (Game|SpawnActorfromClass (Variables|Default|GetDropCubeType) (Transformation|GetActorTransform (Components|GetOwner)) "AlwaysSpawn" 0 0))
        (Variables|Default|SetSpawnedCube _returnvalue)
        (Utilities|FlowControl|Delay (+ (* (Math|Random|RandomFloat) 5.0) 5.0))
        (if (Utilities|IsValid (Variables|Default|GetSpawnedCube))
          (if (Ability|HasAuthority (Variables|Default|GetSpawnedCube))
            (CallFunction|PrintStringwithOwnerEntityIdandCubeName "Has authority to set self destruct" (Variables|Default|GetSpawnedCube))
            (else
              (CallFunction|PrintStringwithOwnerEntityIdandCubeName "Has no authority to set self destruct" (Variables|Default|GetSpawnedCube))))
          (Default|OnSetShouldSelfDestruct (Variables|Default|GetSpawnedCube))
          (Utilities|FlowControl|Delay 0.2)
          (CallFunction|ServerCubeLogic)
          (else
            (CallFunction|PrintStringwithOwnerEntityId "GetSpawnedCube is invalid")))
        (else
          (CallFunction|PrintStringwithOwnerEntityId "Want to create DropCube but without authority"))))))

(event EventEndPlay
  (params (EndPlayReason :type EEndPlayReason%20Enum :default "Destroyed"))
  (bind _spawnedcube (Variables|Default|GetSpawnedCube))
  (CallFunction|PrintStringwithOwnerEntityId "lost authority, force set should self destruct")
  (if (Utilities|IsValid _spawnedcube)
    (Default|OnSetShouldSelfDestruct _spawnedcube)))

(event EventAuthorityLost
  (bind _spawnedcube (Variables|Default|GetSpawnedCube))
  (CallFunction|PrintStringwithOwnerEntityId "lost authority, force set should self destruct")
  (if (Utilities|IsValid _spawnedcube)
    (Default|OnSetShouldSelfDestruct _spawnedcube)))

(fn PrintStringwithOwnerEntityId
  (params (String :type String))
  (bind _returnvalue (Components|GetOwner))
  (Development|PrintString (Utilities|String|Append (Utilities|GetDisplayName _returnvalue) ",EntityId:" (Class|SpatialStatics|GetActorEntityIdasString _returnvalue) "," String)))

(fn PrintStringwithOwnerEntityIdandCubeName
  (params (String :type String) (CurrentCube :type Actor%20Object%20Reference))
  (bind _returnvalue (Components|GetOwner))
  (Development|PrintString (Utilities|String|Append (Utilities|GetDisplayName _returnvalue) ",EntityId:" (Class|SpatialStatics|GetActorEntityIdasString _returnvalue) "," String ",Cube:" (Utilities|GetDisplayName CurrentCube))))