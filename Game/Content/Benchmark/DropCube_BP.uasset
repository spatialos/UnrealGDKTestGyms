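; Benchmark drop cube actor that handles its own cross-server destruction under spatial networking.
; A cross-server self-destruct event destroys the cube on authority; elsewhere it prints an error, throttled by a DoOnce with a delayed reset.
; BeginPlay flags authority as received only when spatial networking is off.
; AuthorityGained just prints a message, and the flag is never read in these graphs.
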(event Custom|CrossServerSetShouldSelfDestruct
  (Networking|SwitchHasAuthority
    (:Authority
      ;[1 1 1 1 12] As destroy can be issued at any point, including when the runtime is creating the Actor, cache destroy command and execute once in authority
      (Actor|DestroyActor))
    (:Remote
      (Utilities|FlowControl|DoOnce false :!label _label
        (:Completed
          (Development|PrintString "Error: No authority to delete cube")
          (Utilities|FlowControl|Delay 2e+01)
          (goto _label Reset))))))

(event EventBeginPlay
  (if (not (Class|SpatialStatics|IsSpatialNetworkingEnabled))
    (Variables|Default|SetHasRecievedAuth true)))

(event Collision|EventActorBeginOverlap
  (params (OtherActor :type Actor%20Object%20Reference)))

(event EventTick
  (params (DeltaSeconds :type Float%20%28single-precision%29)))

(event EventAuthorityGained
  (Development|PrintString "Drop Cube Authority Gained"))

(fn ConstructionScript)