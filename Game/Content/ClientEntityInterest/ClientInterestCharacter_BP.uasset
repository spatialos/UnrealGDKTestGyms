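; Character Blueprint for what appears to be a SpatialOS client entity interest test, visualizing its net cull distance on non-server instances.
; On BeginPlay it reveals the NCD component, scaled flat in X and Y from the square root of NetCullDistanceSquared.
; It logs authority gains and losses, and the mouse wheel adjusts camera boom length.
; The ServerProperty OnRep ends a latency trace on remote instances and prints whether it succeeded.
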(event EventBeginPlay
  (bind _netculldistancesquared (Variables|Default|GetNetCullDistanceSquared))
  (bind _returnvalue (Math|Float|Sqrt _netculldistancesquared))
  (bind _returnvalue_2 (/ _returnvalue 5e+01))
  (|CallParentFunction)
  (if (not (Networking|IsServer))
    (Rendering|SetVisibility (Variables|Default|GetNCD) true true)
    (Transformation|SetWorldScale3D (Variables|Default|GetNCD) (Math|Vector|MakeVector _returnvalue_2 _returnvalue_2 0.0))))

(event EventAuthorityGained
  (|CallParentFunction)
  (Class|SpatialStatics|PrintStringSpatial (Utilities|String|Append (Utilities|GetDisplayName self) ": Gained authority")))

(event EventAuthorityLost
  (|CallParentFunction)
  (Class|SpatialStatics|PrintStringSpatial (Utilities|String|Append (Utilities|GetDisplayName self) ": Lost authority")))

(event Input|MouseEvents|MouseWheelAxis
  (params (AxisValue :type Float%20%28single-precision%29))
  (bind _cameraboom (Variables|Default|GetCameraBoom))
  (Variables|/Script/Engine.SpringArmComponent|SetTargetArmLength _cameraboom (+ (* AxisValue -1e+02) (Variables|/Script/Engine.SpringArmComponent|GetTargetArmLength _cameraboom))))

(fn ConstructionScript)

(fn OnRepServerProperty
  (Networking|SwitchHasAuthority
    (:Remote
      (bind _returnvalue (Class|SpatialLatencyTracer|EndLatencyTrace (Variables|Default|GetServerProperty)))
      (if _returnvalue
        (Development|PrintString "Successfully finished component update trace")
        (else
          (Development|PrintString "Failed to end property update trace"))))))