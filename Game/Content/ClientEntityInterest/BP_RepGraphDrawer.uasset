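; Debug-style actor that spawns BP_RepGraphRegion actors, apparently to visualize replication graph regions, on non-server instances only.
; On BeginPlay it derives an origin from WorldRootOffset and loops over a count of WorldRootOffset squared divided by RegionSize.
; Quotient and remainder of each index set X and Y at fixed height.
; The divisor is that same total, so regions line up along Y rather than forming a square grid.
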(event EventBeginPlay
  (bind _worldrootoffset (Variables|Default|GetWorldRootOffset))
  (bind _worldrootoffset_2 (Variables|Default|GetWorldRootOffset))
  (bind _regionsize (Variables|Default|GetRegionSize))
  (bind _regionsize_2 (Variables|Default|GetRegionSize))
  (bind _returnvalue (Math|Float|Square _worldrootoffset_2))
  (bind _returnvalue_2 (/ _worldrootoffset 2.0))
  (bind _returnvalue_3 (Math|Float|Division(WholeandRemainder) _returnvalue _regionsize))
  (if (not (Networking|IsServer))
    (Variables|Default|SetWorldRoot (+ (- (Math|Vector|VectorZero) (Math|Vector|MakeVector _worldrootoffset _worldrootoffset 0.0)) (Math|Vector|MakeVector _returnvalue_2 _returnvalue_2 0.0)))
    (for _index (range 0 _returnvalue_3)
      (Game|SpawnActorfromClass "/Game/ClientEntityInterest/BP_RepGraphRegion.BP_RepGraphRegion_C" (Math|Transform|MakeTransform (+ (Variables|Default|GetWorldRoot) (Math|Vector|MakeVector (* (.ReturnValue (Math|Float|Division(WholeandRemainder) (Math|Conversions|ToFloat(Integer) _index) (Math|Conversions|ToFloat(Integer) _returnvalue_3))) _regionsize_2) (* (.Remainder (Math|Float|Division(WholeandRemainder) (Math|Conversions|ToFloat(Integer) _index) (Math|Conversions|ToFloat(Integer) _returnvalue_3))) _regionsize_2) 2e+02)) "0, 0, 0" "1,1,1") "AlwaysSpawn" self (Variables|Default|GetRegionSize) 0))))

(event Collision|EventActorBeginOverlap
  (params (OtherActor :type Actor%20Object%20Reference)))

(event EventTick
  (params (DeltaSeconds :type Float%20%28single-precision%29)))

(fn ConstructionScript)