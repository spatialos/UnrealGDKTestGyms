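; Simulated player character for benchmarking that hands its pawn over to an AI controller.
; After BeginPlay it waits a fixed delay, then proceeds only if the pawn is locally controlled.
; It spawns a SimulatedPlayerAIController_BP owned by the current controller and has it possess the pawn, replacing that controller.
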(event EventBeginPlay
  (|CallParentFunction)
  (Utilities|FlowControl|Delay 8.0)
  (if (Pawn|IsLocallyControlled)
    (bind _returnvalue (Game|SpawnActorfromClass "/Game/Characters/SimulatedPlayers/SimulatedPlayerAIController_BP.SimulatedPlayerAIController_BP_C" (Math|Transform|MakeTransform "0, 0, 0" "0, 0, 0" "1,1,1") "AlwaysSpawn" (Pawn|GetController) 0))
    (Pawn|Possess _returnvalue self)))

(event Collision|EventActorBeginOverlap
  (params (OtherActor :type Actor%20Object%20Reference))
  (|CallParentFunction OtherActor) ; This node is disabled and will not be called.\nDrag off pins to build functionality.
)

(event EventTick
  (params (DeltaSeconds :type Float%20%28single-precision%29))
  (|CallParentFunction DeltaSeconds) ; This node is disabled and will not be called.\nDrag off pins to build functionality.
)

(fn ConstructionScript
  (|CallParentFunction))