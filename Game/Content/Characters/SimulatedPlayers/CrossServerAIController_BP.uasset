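; AI controller for simulated players that starts their behavior tree, named for cross-server use.
; On BeginPlay it initializes the simulated player blackboard, seeds both TargetA and TargetB with the controller's own root component location, then runs the simulated player behavior tree.
; Possess and UnPossess only print the affected pawn for debugging, and Tick is unused.
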(event EventBeginPlay
  (bind _rootcomponent (Variables|Transformation|GetRootComponent))
  (bind _returnvalue (Transformation|GetWorldLocation _rootcomponent))
  (bind _blackboardcomponent (Class|AIController|UseBlackboard "/Game/Characters/SimulatedPlayers/SimulatedPlayerBlackboard_BP.SimulatedPlayerBlackboard_BP"))
  (AI|Components|Blackboard|SetValueasVector _blackboardcomponent (Utilities|Name|MakeLiteralName "TargetA") _returnvalue)
  (AI|Components|Blackboard|SetValueasVector _blackboardcomponent (Utilities|Name|MakeLiteralName "TargetB") _returnvalue)
  (AI|RunBehaviorTree "/Game/Characters/SimulatedPlayers/SimulatedPlayerBehaviorTree_BP.SimulatedPlayerBehaviorTree_BP"))

(event EventTick
  (params (DeltaSeconds :type Float%20%28single-precision%29)))

(event EventPossess
  (params (PossessedPawn :type Pawn%20Object%20Reference))
  (Development|PrintString (Utilities|String|ToString(Text) (Utilities|Text|FormatText "OnPossess {Pawn}" (Utilities|Text|ToText(Object) PossessedPawn)))))

(event EventUnPossess
  (params (UnpossessedPawn :type Pawn%20Object%20Reference))
  (Development|PrintString (Utilities|String|ToString(Text) (Utilities|Text|FormatText "OnUnPossess {Pawn}" (Utilities|Text|ToText(Object) UnpossessedPawn)))))

(fn ConstructionScript)