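; AI controller Blueprint for offloaded simulated-player NPCs.
; On BeginPlay it sets up the simulated player blackboard and runs the simulated player behavior tree, which holds the actual decision logic.
; Possess and UnPossess events only print debug messages naming the affected pawn.
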(event EventBeginPlay
  (Class|AIController|UseBlackboard "/Game/Characters/SimulatedPlayers/SimulatedPlayerBlackboard_BP.SimulatedPlayerBlackboard_BP")
  (AI|RunBehaviorTree "/Game/Characters/SimulatedPlayers/SimulatedPlayerBehaviorTree_BP.SimulatedPlayerBehaviorTree_BP"))

(event EventPossess
  (params (PossessedPawn :type Pawn%20Object%20Reference))
  (Development|PrintString (Utilities|String|ToString(Text) (Utilities|Text|FormatText "OnPossess {Pawn}" (Utilities|Text|ToText(Object) PossessedPawn)))))

(event EventUnPossess
  (params (UnpossessedPawn :type Pawn%20Object%20Reference))
  (Development|PrintString (Utilities|String|ToString(Text) (Utilities|Text|FormatText "OnUnPossess {Pawn}" (Utilities|Text|ToText(Object) UnpossessedPawn)))))

(fn ConstructionScript)