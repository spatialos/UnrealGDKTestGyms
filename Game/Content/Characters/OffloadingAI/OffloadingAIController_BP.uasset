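; AI controller for the OffloadingAI character that starts its behavior tree when it possesses a pawn.
; On possess it seeds the blackboard with the character's Enraged flag, a random reachable point within a wide radius as TargetA, and the pawn's location as TargetB.
; It then sets IsSettingValues to true and prints the pawn's local network role for debugging.
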(event EventPossess
  (params (PossessedPawn :type Pawn%20Object%20Reference))
  (bind _blackboard (Variables|Default|GetBlackboard))
  (AI|RunBehaviorTree "/Game/Characters/OffloadingAI/OffloadingAI_BT.OffloadingAI_BT")
  (AI|Components|Blackboard|SetValueasBool _blackboard (Utilities|Name|MakeLiteralName "Enraged") (Variables|/Game/Characters/OffloadingAI/OffloadingAICharacter_BP.OffloadingAICharacter_BP_C|GetEnraged (.AsOffloading%20AICharacter%20BP (Utilities|Casting|CastToOffloadingAICharacter_BP PossessedPawn))))
  (AI|Components|Blackboard|SetValueasVector _blackboard (Utilities|Name|MakeLiteralName "TargetA") (.RandomLocation (AI|Navigation|GetRandomReachablePointinRadius (Transformation|GetActorLocation (Pawn|GetControlledPawn)) 1e+04 0 0)))
  (AI|Components|Blackboard|SetValueasVector _blackboard (Utilities|Name|MakeLiteralName "TargetB") (Transformation|GetActorLocation (Pawn|GetControlledPawn)))
  (AI|Components|Blackboard|SetValueasBool _blackboard (Utilities|Name|MakeLiteralName "IsSettingValues") true)
  (Development|PrintText (Utilities|Text|ToText(Name) (Utilities|Name|EnumtoName (Networking|GetLocalRole (Pawn|GetControlledPawn))))))

(fn ConstructionScript)