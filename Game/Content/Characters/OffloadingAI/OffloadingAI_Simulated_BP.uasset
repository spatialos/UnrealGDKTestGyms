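; OffloadingAI_Simulated_BP is a character Blueprint that hands itself from a player controller to an AI controller on the local machine.
; Shortly after BeginPlay, if a locally controlled player controller holds it outside a dedicated server, it spawns OffloadingAIController_BP owned by that controller.
; The AI controller possesses the character, then the old player controller's view target returns to it after a brief delay.
; The AuthorityGained event is an empty stub.
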(event EventBeginPlay
  (bind _returnvalue (Pawn|GetController))
  (bind (_asplayer_controller _bsuccess) (Utilities|Casting|CastToPlayerController _returnvalue))
  (|CallParentFunction)
  (if _bsuccess
    (Utilities|FlowControl|Delay 3.0)
    (if (and (Pawn|IsLocallyControlled) (not (Networking|IsDedicatedServer)))
      (Development|PrintText (Utilities|Text|ToText(Object) _asplayer_controller))
      (bind _returnvalue_2 (Game|SpawnActorfromClass "/Game/Characters/OffloadingAI/OffloadingAIController_BP.OffloadingAIController_BP_C" (Transformation|GetActorTransform) "AlwaysSpawn" _asplayer_controller 0))
      (Variables|Default|SetOldPC _asplayer_controller)
      (Pawn|Possess _returnvalue_2 self)
      (Utilities|FlowControl|Delay 1.0)
      (Game|Player|SetViewTargetwithBlend (Variables|Default|GetOldPC) self 0.0 "VTBlend_Linear" 0.0 false))))

(event EventAuthorityGained)

(fn ConstructionScript
  (|CallParentFunction))