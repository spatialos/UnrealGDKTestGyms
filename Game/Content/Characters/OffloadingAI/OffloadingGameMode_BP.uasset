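; Game mode for the offloading AI setup that drives the NPC count from a worker flag.
; On authority, BeginPlay starts a looping one-second timer to poll the flag through CheckNumNPCsWorkerFlag.
; A changed flag value is cached and written to NumNPCs, whose RepNotify passes the new count to the first AISpawner_BP found in the world.
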(event Custom|CheckNumNPCsWorkerFlag
  (bind (_outflagvalue _returnvalue) (Class|SpatialStatics|GetWorkerFlag (Variables|Default|GetNumNPCsWorkerFlagName)))
  (if _returnvalue
    (if (!= (Math|Conversions|ToInteger(Byte) _outflagvalue) (Variables|Default|GetWorkerFlagValue))
      (Variables|Default|SetWorkerFlagValue (Math|Conversions|ToInteger(Byte) _outflagvalue))
      (Variables|Default|SetNumNPCs (Math|Conversions|ToInteger(Byte) _outflagvalue)))))

(event EventBeginPlay
  (Networking|SwitchHasAuthority
    (:Authority
      (Utilities|Time|SetTimerbyEvent (EventDispatchers|CreateEvent :!event Custom|CheckNumNPCsWorkerFlag) 1.0 true))))

(fn ConstructionScript)

(fn OnRepNumNPCs
  (bind _outactors (Actor|GetAllActorsOfClass "/Game/Characters/OffloadingAI/AISpawner_BP.AISpawner_BP_C"))
  (if (> (Utilities|Array|Length _outactors) 0)
    (Default|UpdateAINumber (Utilities|Array|Get(acopy) _outactors) (Variables|Default|GetNumNPCs))))