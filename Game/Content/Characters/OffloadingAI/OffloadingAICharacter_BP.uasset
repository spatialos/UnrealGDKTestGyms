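; Multi-server (Spatial) character, AI or player controlled, that scores from food and can randomly become enraged.
; Replicated enrage state changes size, material, speed, camera and AI blackboard; enraged characters kill others they overlap.
; Death resets score, hides and relocates the character until a timed respawn, showing local players a death screen.
; Servers not owning its actor group disable movement; gaining authority spawns the default controller.
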(event OnComponentBeginOverlap(EnrageSphere)
  (params (OverlappedComponent :type Primitive%20Component%20Object%20Reference) (OtherActor :type Actor%20Object%20Reference) (OtherComp :type Primitive%20Component%20Object%20Reference) (OtherBodyIndex :type Integer) (bFromSweep :type Boolean) (SweepResult :type Hit%20Result%20Structure%20%28by%20ref%29))
  (Networking|SwitchHasAuthority
    (:Authority
      (if (!= self OtherActor)
        (bind _asoffloading_aicharacter_bp (Utilities|Casting|CastToOffloadingAICharacter_BP OtherActor))
        (if (Variables|Default|GetEnraged)
          (Utilities|FlowControl|DoOnce false :!label _label
            (:Completed
              (CallFunction|Kill _asoffloading_aicharacter_bp)
              (CallFunction|AddScore false)
              (goto _label Reset))))))))

(event Custom|AddScore
  (params (FromFood :type Boolean))
  (Variables|Default|SetScore (+ (Variables|Default|GetScore) 1))
  (if FromFood
    (if (Math|Random|RandomBoolwithWeight (Variables|Default|GetEnrageChance))
      (Variables|Default|SetEnraged true)
      (Utilities|Time|SetTimerbyEvent (delegate Custom|StopEnrage) (Variables|Default|GetEnrageDuration)))))

(event Custom|StopEnrage
  (Variables|Default|SetEnraged false))

(event Custom|Kill
  (bind _asoffloading_aicontroller_bp (Utilities|Casting|CastToOffloadingAIController_BP (Pawn|GetController))
    (:then
      (Actor|DestroyActor _asoffloading_aicontroller_bp))
    (:CastFailed
      _))
  (Pawn|Components|CharacterMovement|DisableMovement (Variables|Character|GetCharacterMovement))
  (Variables|Default|SetScore 0)
  (Variables|Default|SetEnraged false)
  (Variables|Default|SetDead true)
  (Rendering|SetActorHiddenInGame false)
  (Transformation|SetActorLocation (+ (.RandomLocation (AI|Navigation|GetRandomReachablePointinRadius (Transformation|GetActorLocation) 5e+04 0 0)) "0, 0,-600.000000") false false)
  (Rendering|SetActorHiddenInGame true)
  (Utilities|Time|SetTimerbyEvent (EventDispatchers|CreateEvent :!event Custom|Respawn) (Variables|Default|GetRespawnTime)))

(event Custom|Respawn
  (bind _returnvalue (Transformation|GetActorLocation))
  (if (not (Pawn|IsPlayerControlled))
    (Pawn|SpawnDefaultController))
  (Transformation|SetActorLocation (Math|Vector|MakeVector (.x _returnvalue) (.y _returnvalue) 5e+02) false false)
  (Pawn|Components|CharacterMovement|SetMovementMode (Variables|Character|GetCharacterMovement) "MOVE_Walking" 0)
  (Rendering|SetActorHiddenInGame false)
  (Variables|Default|SetDead false))

(event EventBeginPlay
  (if (and (Networking|IsServer) (not (Class|SpatialStatics|IsActorGroupOwnerforActor self)))
    (Class|SpatialStatics|PrintTextSpatial (Utilities|Text|FormatText "Disabling non-auth movement component for {Name}" (Utilities|Text|ToText(Object) self)))
    (Components|Activation|Deactivate (Variables|Character|GetCharacterMovement))))

(event EventAuthorityGained
  (Pawn|SpawnDefaultController))

(fn ConstructionScript
  (CallFunction|UpdateEnragedState))

(fn OnRepScore)

(fn OnRepEnraged
  (CallFunction|UpdateEnragedState))

(fn UpdateEnragedState
  (Transformation|SetActorScale3D (select (Variables|Default|GetEnraged) "2.000000,2.000000,2.000000" "1.000000,1.000000,1.000000"))
  (Rendering|Material|SetMaterial (Variables|Character|GetMesh) 0 (select (Variables|Default|GetEnraged) (Variables|Default|GetEnragedMaterial) (Variables|Default|GetDefaultMaterial)))
  (Variables|/Script/Engine.CharacterMovementComponent|SetMaxWalkSpeed (Variables|Character|GetCharacterMovement) (select (Variables|Default|GetEnraged) 1.2e+03 6e+02))
  (Variables|/Script/Engine.CharacterMovementComponent|SetMaxAcceleration (Variables|Character|GetCharacterMovement) (select (Variables|Default|GetEnraged) 4096.0 2048.0))
  (Variables|/Script/Engine.SpringArmComponent|SetTargetArmLength (Variables|Default|GetCameraBoom) (select (Variables|Default|GetEnraged) 6e+02 3e+02))
  (if (not (Pawn|IsPlayerControlled))
    (bind _asoffloading_aicontroller_bp (Utilities|Casting|CastToOffloadingAIController_BP (Pawn|GetController)))
    (AI|Components|Blackboard|SetValueasBool (Variables|/Script/AIModule.AIController|GetBlackboard _asoffloading_aicontroller_bp) (Utilities|Name|MakeLiteralName "Enraged") (Variables|Default|GetEnraged))
    (Class|CharacterMovementComponent|SetAvoidanceEnabled (Variables|Character|GetCharacterMovement) (not (Variables|Default|GetEnraged)))))

(fn OnRepDead
  (bind _returnvalue (Pawn|GetController))
  (Utilities|IsValid _returnvalue
    (:Is%20Valid
      (if (and (Pawn|IsLocalPlayerController _returnvalue) (not (Networking|IsDedicatedServer)))
        (if (Variables|Default|GetDead)
          (bind _returnvalue_2 (UserInterface|CreateWidget "/Game/Characters/OffloadingAI/UI_DeathScreen.UI_DeathScreen_C" 0 (Math|Float|Truncate (Variables|Default|GetRespawnTime))))
          (bind _output_get (Variables|Default|SetDeathUI _returnvalue_2))
          (UserInterface|Viewport|AddtoViewport _output_get 0)
          (else
            (Utilities|IsValid (Variables|Default|GetDeathUI)
              (:Is%20Valid
                (Widget|RemovefromParent (Variables|Default|GetDeathUI))))))))))