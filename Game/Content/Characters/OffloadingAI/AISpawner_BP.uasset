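; AISpawner_BP adjusts the number of spawned AI characters to match a target count passed to UpdateAINumber.
; It caches all PlayerStart actors on BeginPlay and spawns missing characters at random ones, adjusting for collision but always spawning.
; To reduce the count, each loop pass either destroys the first tracked AI or, if invalid, removes its entry, so destruction and array removal happen on separate passes.
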(event EventBeginPlay
  (bind _outactors (Actor|GetAllActorsOfClass "/Script/Engine.PlayerStart"))
  (Variables|Default|SetPlayerStarts _outactors))

(fn ConstructionScript)

(fn UpdateAINumber
  (params (TargetNumber :type Integer))
  (bind _spawnedai (Variables|Default|GetSpawnedAI))
  (bind _output (Utilities|Array|Get(acopy) _spawnedai))
  (LocalVariables|SetTarget TargetNumber)
  (LocalVariables|SetCurrent (Utilities|Array|Length (Variables|Default|GetSpawnedAI)))
  (Math|Integer|CompareInt (LocalVariables|GetTarget) (LocalVariables|GetCurrent)
    (:>
      ;[1 1 1] Spawn New NPCs
      (for _index (range 1 (- (LocalVariables|GetTarget) (LocalVariables|GetCurrent)))
        (bind _returnvalue (Game|SpawnActorfromClass (Variables|Default|GetAICharacterClass) (Transformation|GetActorTransform (Utilities|Array|Get(acopy) (Variables|Default|GetPlayerStarts) (Math|Random|RandomIntegerinRange 0 (- (Utilities|Array|Length (Variables|Default|GetPlayerStarts)) 1)))) "AdjustIfPossibleButAlwaysSpawn" 0 0))
        (Utilities|Array|Add (Variables|Default|GetSpawnedAI) _returnvalue)))
    (:<
      ;[1 1 1] Delete NPCs
      (for _index_2 (range 0 (- (LocalVariables|GetCurrent) (LocalVariables|GetTarget)))
        (Utilities|IsValid _output
          (:Is%20Valid
            (Actor|DestroyActor _output))
          (:Is%20Not%20Valid
            (Utilities|Array|RemoveIndex (Variables|Default|GetSpawnedAI))))))))