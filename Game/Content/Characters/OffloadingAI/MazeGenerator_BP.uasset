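; Maze generator actor that builds instanced walls over a metre-sized area and scatters actors across its grid.
; GenerateMaze seeds a random stream, then adds outer and inner walls.
; SpawnDistributedActors resets the stream, destroys earlier spawns and places each ActorDistributions entry on grid cells, tracking used positions.
; Spawned actors carry GeneratedTag, so the construction script can re-collect them for later clearing.
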(event EventBeginPlay)

(event Collision|EventActorBeginOverlap
  (params (OtherActor :type Actor%20Object%20Reference)))

(event EventTick
  (params (DeltaSeconds :type Float%20%28single-precision%29)))

(fn ConstructionScript
  (bind _outactors (Actor|GetAllActorswithTag (Variables|Default|GetGeneratedTag)))
  (for _array_element _outactors
    (Utilities|Array|AddUnique (Variables|Default|GetSpawnedActors) _array_element)))

(fn GenerateMaze
  (Components|InstancedStaticMesh|ClearInstances (Variables|Default|GetWalls))
  (Math|Random|SetRandomStreamSeed (Variables|Default|GetRandomStream) (Variables|Default|GetSeed))
  (CallFunction|AddOuterWalls)
  (Class|MazeGenerator|AddInnerWalls))

(fn AddOuterWalls
  (Utilities|FlowControl|Sequence
    (:then_0
      (Class|MazeGenerator|AddWall 0.0 (/ (Variables|Default|GetWidthInMetres) 2.0) (Variables|Default|GetLengthInMetres) false)
      (Class|MazeGenerator|AddWall 0.0 (/ (Variables|Default|GetWidthInMetres) -2.0) (Variables|Default|GetLengthInMetres) false))
    (:then_1
      (Class|MazeGenerator|AddWall (/ (Variables|Default|GetLengthInMetres) 2.0) 0.0 (Variables|Default|GetWidthInMetres) true)
      (Class|MazeGenerator|AddWall (/ (Variables|Default|GetLengthInMetres) -2.0) 0.0 (Variables|Default|GetWidthInMetres) true))))

(fn ClearMaze
  (Components|InstancedStaticMesh|ClearInstances (Variables|Default|GetWalls)))

(fn SpawnDistributedActors
  (bind _randomstream (Variables|Default|GetRandomStream))
  (Class|KismetMathLibrary|ResetRandomStream (Variables|Default|GetRandomStream))
  (for _array_element (Variables|Default|GetSpawnedActors)
    (Actor|DestroyActor _array_element))
  (for _array_element_2 (Variables|Default|GetActorDistributions)
    (for _index (range 1 (.NumberToSpawn (Utilities|Struct|BreakActorDistribution _array_element_2)))
      (LocalVariables|SetNextSpawnPosition (Utilities|Struct|MakeIntVector -1 -1 -1))
      (while (Utilities|Set|Contains (LocalVariables|GetSpawnPositions) (LocalVariables|GetNextSpawnPosition))
        (LocalVariables|SetNextSpawnPosition (Utilities|Struct|MakeIntVector (Math|Random|RandomIntegerinRangefromStream 0 (- (Variables|Default|GetRows) 1) _randomstream) (Math|Random|RandomIntegerinRangefromStream 0 (- (Variables|Default|GetCols) 1) _randomstream) 0)))
      (Utilities|Set|Add (LocalVariables|GetSpawnPositions) (LocalVariables|GetNextSpawnPosition))
      (bind _returnvalue (Game|SpawnActorfromClass (.ActorClass (Utilities|Struct|BreakActorDistribution _array_element_2)) (Math|Transform|MakeTransform (+ (.LocalOffset (Utilities|Struct|BreakActorDistribution _array_element_2)) (CallFunction|ToWorldSpace (LocalVariables|GetNextSpawnPosition))) "0, 0, 0" "1,1,1") "AlwaysSpawn" 0 0))
      (Utilities|Array|AddUnique (Variables|/Script/Engine.Actor|GetTags _returnvalue) (Variables|Default|GetGeneratedTag))
      (Utilities|Array|Add (Variables|Default|GetSpawnedActors) _returnvalue))))

(fn ToWorldSpace
  (params (GridPosition :type Int%20Vector%20Structure))
  (bind _returnvalue (Transformation|GetActorLocation))
  (bind _returnvalue_2 (Math|Conversions|ToVector(Float) GridPosition))
  (bind _widthinmetres (Variables|Default|GetWidthInMetres))
  (bind _lengthinmetres (Variables|Default|GetLengthInMetres))
  (bind _lengthinmetres_2 (Variables|Default|GetLengthInMetres))
  (bind _rows (Variables|Default|GetRows))
  (bind _widthinmetres_2 (Variables|Default|GetWidthInMetres))
  (bind _cols (Variables|Default|GetCols))
  (bind _returnvalue_3 (Math|Conversions|ToFloat(Integer) _cols))
  (bind _returnvalue_4 (Math|Conversions|ToFloat(Integer) _rows))
  (bind _returnvalue_5 (* _lengthinmetres 5e+01))
  (bind _returnvalue_6 (* _widthinmetres 5e+01))
  (bind _returnvalue_7 (/ _widthinmetres_2 _returnvalue_3))
  (bind _returnvalue_8 (/ _lengthinmetres_2 _returnvalue_4))
  (bind _returnvalue_9 (- _returnvalue (Math|Vector|MakeVector _returnvalue_5 _returnvalue_6 0.0)))
  (bind _returnvalue_10 (* _returnvalue_7 1e+02))
  (bind _returnvalue_11 (* _returnvalue_8 1e+02))
  (bind _returnvalue_12 (/ _returnvalue_11 2.0))
  (bind _returnvalue_13 (/ _returnvalue_10 2.0))
  (bind _returnvalue_14 (* _returnvalue_2 (Math|Vector|MakeVector _returnvalue_11 _returnvalue_10 0.0)))
  (bind _returnvalue_15 (+ _returnvalue_14 _returnvalue_9 (Math|Vector|MakeVector _returnvalue_12 _returnvalue_13 0.0)))
  (return (Math|Vector|MakeVector (.x _returnvalue_15) (.y _returnvalue_15) (.z (Transformation|GetActorLocation)))))

(fn ClearDistributedActors
  (for _array_element (Variables|Default|GetSpawnedActors)
    (Actor|DestroyActor _array_element)))