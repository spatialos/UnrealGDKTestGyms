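; Player character Blueprint that can turn a client-owned pawn into an AI-driven simulated player.
; On client ownership gain, a DoOnce runs the simulated-player check, then pauses movement component ticking for a timed delay.
; It then spawns a SimulatedPlayerAIController_BP to possess the character and points the original player controller's view back at it.
; Ownership loss only prints a debug message.
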(event EventClientOwnershipGained
  (bind _returnvalue (Pawn|GetController))
  (Development|PrintString "Client ownership gained")
  (Utilities|FlowControl|DoOnce false
    (:Completed
      (if (Class|SimPlayerBPFunctionLibrary|IsSimulatedPlayer)
        (Utilities|FlowControl|Delay 0.2)
        (Components|Tick|SetComponentTickEnabled (Variables|Character|GetCharacterMovement) false)
        (Utilities|FlowControl|Delay 8.0)
        (Components|Tick|SetComponentTickEnabled (Variables|Character|GetCharacterMovement) true)
        (bind _asplayer_controller (Utilities|Casting|CastToPlayerController _returnvalue))
        (Variables|Default|SetOldPC _asplayer_controller)
        (bind _returnvalue_2 (Game|SpawnActorfromClass "/Game/Characters/SimulatedPlayers/SimulatedPlayerAIController_BP.SimulatedPlayerAIController_BP_C" (Math|Transform|MakeTransform (Transformation|GetActorLocation _returnvalue) "0, 0, 0" "1,1,1") "AlwaysSpawn" _returnvalue 0))
        (Components|Tick|SetComponentTickEnabled (Variables|Character|GetCharacterMovement) true)
        (Pawn|Possess _returnvalue_2 self)
        (Utilities|FlowControl|Delay 1.0)
        (Game|Player|SetViewTargetwithBlend (Variables|Default|GetOldPC) self 0.0 "VTBlend_Linear" 0.0 false)
        (Development|PrintString "AI setup")))))

(event EventClientOwnershipLost
  (Development|PrintString "Client ownership lost"))

(fn ConstructionScript)