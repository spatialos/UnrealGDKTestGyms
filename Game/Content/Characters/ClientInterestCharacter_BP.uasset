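; A SpatialOS character Blueprint that visualizes net cull distance and logs authority changes and latency trace results.
; On non-server instances, BeginPlay shows the NCD component and flattens it, scaled in X and Y from the square root of NetCullDistanceSquared.
; AuthorityGained and AuthorityLost print the actor's name with the change.
; ServerProperty's RepNotify ends a latency trace on the remote side and prints success or failure.
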(event EventBeginPlay
  (bind _netculldistancesquared (Variables|Default|GetNetCullDistanceSquared))
  (bind _returnvalue (Math|Float|Sqrt _netculldistancesquared))
  (bind _returnvalue_2 (/ _returnvalue 5e+01))
  (|CallParentFunction)
  (if (not (Networking|IsServer))
    (Rendering|SetVisibility (Variables|Default|GetNCD) true true)
    (Transformation|SetWorldScale3D (Variables|Default|GetNCD) (Math|Vector|MakeVector _returnvalue_2 _returnvalue_2 0.0))))

(event EventAuthorityGained
  (|CallParentFunction)
  (Class|SpatialStatics|PrintStringSpatial (Utilities|String|Append (Utilities|GetDisplayName self) ": Gained authority")))

(event EventAuthorityLost
  (|CallParentFunction)
  (Class|SpatialStatics|PrintStringSpatial (Utilities|String|Append (Utilities|GetDisplayName self) ": Lost authority")))

(fn ConstructionScript)

(fn OnRepServerProperty
  (Networking|SwitchHasAuthority
    (:Remote
      (bind _returnvalue (Class|SpatialLatencyTracer|EndLatencyTrace (Variables|Default|GetServerProperty)))
      (if _returnvalue
        (Development|PrintString "Successfully finished component update trace")
        (else
          (Development|PrintString "Failed to end property update trace"))))))