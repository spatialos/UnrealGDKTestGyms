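; PossessableCharacter_BP is a possessable character that exercises SpatialOS authority changes, Gameplay Ability System use and latency tracing.
; Gaining or losing authority prints a spatial log message, and gaining it also applies a counting-grant effect when the character is not yet initialized.
; An ActivateAbility event tries the counting ability with remote activation allowed.
; On non-authoritative instances, the ServerProperty RepNotify ends a latency trace and prints whether it succeeded.
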(event Custom|ActivateAbility
  (Abilities|TryActivateAbilitybyClass (Variables|Default|GetAbilitySystem) "/Game/GASComponents/Ability_Counting.Ability_Counting_C" true))

(event EventAuthorityGained
  (Class|SpatialStatics|PrintStringSpatial (Utilities|String|Append (Utilities|GetDisplayName self) ": Gained authority"))
  (if (Variables|Default|GetInitialized)
    _
    (else
      (GameplayEffects|ApplyGameplayEffectToSelf :self (Variables|Default|GetAbilitySystem) :GameplayEffectClass "/Game/GASComponents/Effect_GrantCounting.Effect_GrantCounting_C")))
  (|CallParentFunction))

(event EventAuthorityLost
  (Class|SpatialStatics|PrintStringSpatial (Utilities|String|Append (Utilities|GetDisplayName self) ": Lost authority")))

(fn ConstructionScript)

(fn OnRepServerProperty
  (Networking|SwitchHasAuthority
    (:Remote
      (bind _returnvalue (Class|SpatialLatencyTracer|EndLatencyTrace (Variables|Default|GetServerProperty)))
      (if _returnvalue
        (Development|PrintString "Successfully finished component update trace")
        (else
          (Development|PrintString "Failed to end property update trace"))))))