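; Player character Blueprint for measuring input-to-network round-trip latency through traced RPCs.
; Releasing I or K begins a latency trace and calls a server RPC, which continues the trace and replies by client or multicast RPC respectively.
; The receiving RPC ends the trace, with debug prints at each hop.
; Releasing J sends a standalone test trace.
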(event Custom|OnInput_ServerRPC
  (params (UseMulticast :type Boolean))
  (if UseMulticast
    (Class|SpatialLatencyTracer|ContinueLatencyTrace self "OnInput_MulticastRPC" "ServerAck > Multicast RPC")
    (Development|PrintString "On Server RPC")
    (CallFunction|OnInputMulticastRPC)
    (else
      (Class|SpatialLatencyTracer|ContinueLatencyTrace self "OnInput_ClientRPC" "ServerAck > Client RPC")
      (Development|PrintString "On Server RPC")
      (CallFunction|OnInputClientRPC))))

(event Custom|OnInput_MulticastRPC
  (Class|SpatialLatencyTracer|EndLatencyTrace)
  (Development|PrintString "On Multicast RPC"))

(event Custom|OnInput_ClientRPC
  (Class|SpatialLatencyTracer|EndLatencyTrace)
  (Development|PrintString "On Client RPC"))

(event EventBeginPlay)

(event Collision|EventActorBeginOverlap
  (params (OtherActor :type Actor%20Object%20Reference)))

(event EventTick
  (params (DeltaSeconds :type Float%20%28single-precision%29)))

(event Input|KeyboardEvents|I
  (params (Key :type Key%20Structure))
  (:Released
    (Development|PrintString "On input")
    (Class|SpatialLatencyTracer|BeginLatencyTrace self "OnInput_ServerRPC" "Input > Server RPC > Client RPC")
    (CallFunction|OnInputServerRPC false)))

(event Input|KeyboardEvents|J
  (params (Key :type Key%20Structure))
  (:Released
    (Class|SpatialLatencyTracer|SendTestTrace)))

(event Input|KeyboardEvents|K
  (params (Key :type Key%20Structure))
  (:Released
    (Development|PrintString "On input")
    (Class|SpatialLatencyTracer|BeginLatencyTrace self "OnInput_ServerRPC" "Input > Server RPC > Multicast RPC")
    (CallFunction|OnInputServerRPC true)))

(fn ConstructionScript)