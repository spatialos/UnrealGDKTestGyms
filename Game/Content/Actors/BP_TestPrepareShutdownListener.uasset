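; Test listener actor that counts prepare-shutdown notifications from the SpatialGameInstance.
; RegisterCallback calls the parent implementation, then casts the game instance and binds an event to OnPrepareShutdown, returning whether both steps succeeded.
; OnPrepareShutdownBlueprint increments BlueprintPrepareShutdownEventCount.
; The event graph holds only an unconnected copy of that increment.
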(fn ConstructionScript)

(fn RegisterCallback
  (bind _returnvalue (|CallParentFunction))
  (if _returnvalue
    (bind _asspatial_game_instance (Utilities|Casting|CastToSpatialGameInstance (Game|GetGameInstance))
      (:then
        (EventDispatchers|BindEventtoOnPrepareShutdown _asspatial_game_instance (EventDispatchers|CreateEvent :!event OnPrepareShutdownBlueprint))
        (return true))
      (:CastFailed
        (return false)))
    (else
      (return false))))

(fn OnPrepareShutdownBlueprint
  (Math|Integer|IncrementInt (Variables|Default|GetBlueprintPrepareShutdownEventCount)))