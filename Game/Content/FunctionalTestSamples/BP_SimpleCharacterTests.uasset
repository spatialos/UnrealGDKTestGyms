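; Simple test character for functional test samples, with health, attack, build and directional movement actions.
; Each Server event forwards to a CrossServer counterpart: attacks damage the victim, builds start construction on the given building, and moves apply a swept, fixed-step location offset.
; Health initialization and damage are authority-gated, and IsDead reports when health reaches zero or below.
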(event Custom|CrossServerAttack
  (params (Damage :type Integer))
  (CallFunction|TakeDamage Damage))

(event Custom|ServerAttack
  (params (Victim :type BP%20Simple%20Character%20Tests%20Object%20Reference))
  (CallFunction|CrossServerAttack Victim (Variables|Const|GetAttackDamage)))

(event Custom|ServerBuild
  (params (Building :type BP%20Test%20Building%20Object%20Reference))
  (CallFunction|CrossServerBuild Building))

(event Custom|CrossServerBuild
  (params (Building :type BP%20Test%20Building%20Object%20Reference))
  (Default|StartBuilding Building))

(event Custom|ServerMoveInDirection
  (params (Direction :type Vector))
  (CallFunction|CrossServerMoveinDirection Direction))

(event Custom|CrossServerMoveInDirection
  (params (Direction :type Vector))
  (Transformation|SetActorLocation (+ (Transformation|GetActorLocation) (* Direction 2e+02)) true false))

(event EventBeginPlay
  (Networking|SwitchHasAuthority
    (:Authority
      (Variables|Replicated|SetHealth (Variables|Const|GetMaxHealth)))))

(fn ConstructionScript)

(fn TakeDamage
  (params (Damage :type Integer))
  (Networking|SwitchHasAuthority
    (:Authority
      (Variables|Replicated|SetHealth (- (Variables|Replicated|GetHealth) Damage)))))

(fn IsDead
  (return (<= (Variables|Replicated|GetHealth) 0)))