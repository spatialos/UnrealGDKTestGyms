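; Actor component that exercises SpatialOS event tracing for RPCs and replicated properties in functional test samples.
; When authority is gained with tracing enabled, a looping timer sends a traced client RPC and increments a traced TestInt.
; Each send creates a new span ID.
; RunOnClient and the TestInt OnRep create spans caused by the active span to log receipt, the OnRep only if the owner has authority.
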(event Custom|StartRun
  (CallFunction|SendClientRPC)
  (CallFunction|UpdateTestInt))

(event Custom|RunOnClient
  (bind (_outuserspanid _returnvalue) (Class|SpatialEventTracerUserInterface|GetActiveSpanId))
  (if _returnvalue
    (bind _returnvalue_2 (Class|SpatialEventTracerUserInterface|CreateSpanIdwithCauses (Utilities|Array|MakeArray _outuserspanid)))
    (Class|SpatialEventTracerUserInterface|TraceEvent _returnvalue_2 (Utilities|Struct|MakeSpatialTraceEvent "user.process_rpc"))))

(event EventAuthorityGained
  (if (Variables|Default|GetUseEventTracing)
    (Utilities|Time|SetTimerbyEvent (delegate Custom|StartRun) 5.0 true)))

(fn OnRepTestInt
  (if (Ability|HasAuthority (Components|GetOwner))
    (bind (_outuserspanid _returnvalue) (Class|SpatialEventTracerUserInterface|GetActiveSpanId))
    (if _returnvalue
      (bind _returnvalue_2 (Class|SpatialEventTracerUserInterface|CreateSpanIdwithCauses (Utilities|Array|MakeArray _outuserspanid)))
      (Class|SpatialEventTracerUserInterface|TraceEvent _returnvalue_2 (Utilities|Struct|MakeSpatialTraceEvent "user.receive_component_property")))))

(fn UpdateTestInt
  (bind _returnvalue (Class|SpatialEventTracerUserInterface|CreateSpanId))
  (Class|SpatialEventTracerUserInterface|TraceEvent _returnvalue (Utilities|Struct|MakeSpatialTraceEvent "user.send_component_property"))
  (Class|SpatialEventTracerUserInterface|TraceProperty self _returnvalue)
  (Math|Integer|IncrementInt (Variables|Default|GetTestInt)))

(fn SendClientRPC
  (bind _returnvalue (Class|SpatialEventTracerUserInterface|CreateSpanId))
  (Class|SpatialEventTracerUserInterface|TraceEvent _returnvalue (Utilities|Struct|MakeSpatialTraceEvent "user.send_rpc"))
  (Class|SpatialEventTracerUserInterface|TraceRPC (EventDispatchers|CreateEvent :!event Custom|RunOnClient) _returnvalue))