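; Functional test sample cube that exercises SpatialGDK event tracing for cross-server RPCs and property replication.
; When tracing is enabled, a looping timer makes the authoritative server send a traced CrossServerRPC to a non-authoritative cube.
; A one-shot timer increments TestInt under a traced property span.
; The RPC handler and TestInt's OnRep emit receive events caused by the active span, linking sender to receiver.
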(event Custom|Toggle)

(event Custom|BeginCrossServerRPC
  (Networking|SwitchHasAuthority
    (:Authority
      (bind _outactors (Actor|GetAllActorsOfClass "BP_EventTracerCrossServerCube_C"))
      (bind _array_element (Utilities|Array|ForEachLoopwithBreak _outactors)
        (:LoopBody
          (if (not (Ability|HasAuthority _array_element))
            (bind _returnvalue (Class|SpatialEventTracerUserInterface|TraceEventBasic "user.send_cross_server_rpc" "" (Utilities|Array|MakeArray)))
            (Class|SpatialEventTracerUserInterface|TraceRPC (delegate Custom|CallCrossRPC) _returnvalue)))))))

(event Custom|CrossServerRPC
  (bind _outuserspanid (Class|SpatialEventTracerUserInterface|GetActiveSpanId))
  (Class|SpatialEventTracerUserInterface|TraceEventBasic "user.receive_cross_server_rpc" "" (Utilities|Array|MakeArray _outuserspanid)))

(event Custom|CallCrossRPC
  (CallFunction|CrossServerRPC (stale Custom|BeginCrossServerRPC _array_element))
  (Utilities|Array|ForEachLoopwithBreak (stale Custom|BeginCrossServerRPC _outactors)) ; enters at Break
)

(event Custom|ModifyCrossServerProperty
  (Networking|SwitchHasAuthority
    (:Authority
      (bind _returnvalue (Class|SpatialEventTracerUserInterface|TraceEvent (Utilities|Struct|MakeSpatialTraceEvent "user.send_cross_server_property")))
      (Class|SpatialEventTracerUserInterface|TraceProperty self _returnvalue)
      (Math|Integer|IncrementInt (Variables|Default|GetTestInt)))))

(event Collision|EventActorBeginOverlap
  (params (OtherActor :type Actor%20Object%20Reference)))

(event EventTick
  (params (DeltaSeconds :type Float%20%28single-precision%29)))

(event EventBeginPlay
  (if (Variables|Default|GetUseEventTracing)
    (Utilities|Time|SetTimerbyEvent (delegate Custom|BeginCrossServerRPC) 5.0 true)
    (Utilities|FlowControl|Delay 0.2)
    (Utilities|Time|SetTimerbyEvent (delegate Custom|ModifyCrossServerProperty) 5.0)))

(fn ConstructionScript)

(fn OnRepTestInt
  (Networking|SwitchHasAuthority
    (:Remote
      (bind (_outuserspanid _returnvalue) (Class|SpatialEventTracerUserInterface|GetActiveSpanId))
      (if _returnvalue
        (Class|SpatialEventTracerUserInterface|TraceEventwithCauses (Utilities|Struct|MakeSpatialTraceEvent "user.receive_cross_server_property") (Utilities|Array|MakeArray _outuserspanid))))))