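; BP_TestBuilding is a functional test sample building that rises over a set build time once construction starts.
; StartBuilding sets a building flag if not yet built, and Tick advances clamped progress, which sets the Scene component's relative height.
; The authority marks IsBuilt at full progress, and its RepNotify snaps remote instances to fully built or unbuilt.
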(event Custom|StartBuilding
  (if (not (Variables|Replicated|GetIsBuilt))
    (Variables|Replicated|SetIsBuilding true)))

(event EventTick
  (params (DeltaSeconds :type Float%20%28single-precision%29))
  (if (Variables|Replicated|GetIsBuilding)
    (CallFunction|SetBuildProgress (+ (Variables|Local|GetBuildProgress) (/ DeltaSeconds (Variables|Const|GetBuildTime))))))

(fn ConstructionScript)

(fn OnRepIsBuilt
  (Networking|SwitchHasAuthority
    (:Remote
      (if (Variables|Replicated|GetIsBuilt)
        (CallFunction|SetBuildProgress 1.0)
        (else
          (CallFunction|SetBuildProgress 0.0))))))

(fn SetBuildProgress
  (params (NewBuildProgress :type Float%20%28single-precision%29))
  (bind _output_get (Variables|Local|SetBuildProgress (Math|Float|Clamp(Float) NewBuildProgress)))
  (Utilities|FlowControl|Sequence
    (:then_0
      (Networking|SwitchHasAuthority
        (:Authority
          (if (>= (Variables|Local|GetBuildProgress) 1.0)
            (Variables|Replicated|SetIsBuilt true)))))
    (:then_1
      (Transformation|SetRelativeLocation (Variables|Default|GetScene) (Math|Vector|MakeVector 0.0 0.0 (* _output_get 1e+02)) false true))))