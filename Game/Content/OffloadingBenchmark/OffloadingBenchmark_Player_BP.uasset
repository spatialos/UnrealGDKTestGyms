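; Player character for the offloading benchmark, with debug keys to drive the test and record performance.
; Keys toggle a client-only HUD, flip an Enraged flag, adjust the GameMode's NPC total, and start a local stat-file capture with a timer alongside a GameMode capture.
; A spectator toggle uses IsSpectating's OnRep to switch flying, collision, visibility and camera boom testing, while Tick applies Space/Ctrl vertical movement.
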(event Custom|Server_ToggleEnrage
  ;[1 1 1] Manually toggle enrage state
  (Variables|Default|SetEnraged (not (Variables|Default|GetEnraged))))

(event Custom|Server_ToggleSpectating
  ;[1 1 1] Toggle spectator mode
  (Variables|Default|SetIsSpectating (not (Variables|Default|GetIsSpectating))))

(event Custom|CaptureServer
  (bind _asoffloading_benchmark_game_mode (Utilities|Casting|CastToOffloadingBenchmark_GameMode (Game|GetGameMode)))
  (Default|DoCapture _asoffloading_benchmark_game_mode))

(event Custom|UpdateNumNPCs
  (params (Delta :type Integer))
  (bind _asoffloading_benchmark_game_mode (Utilities|Casting|CastToOffloadingBenchmark_GameMode (Game|GetGameMode)))
  (Variables|/Script/GDKTestGyms.BenchmarkGymGameModeBase|SetTotalNPCs _asoffloading_benchmark_game_mode (+ (Variables|/Script/GDKTestGyms.BenchmarkGymGameModeBase|GetTotalNPCs _asoffloading_benchmark_game_mode) Delta)))

(event EventTick
  (params (DeltaSeconds :type Float%20%28single-precision%29))
  ;[1 1 1] Add Vertical Velocity when Spectating
  (if (and (Variables|Default|GetIsSpectating) (Pawn|IsLocallyControlled))
    (Pawn|Input|AddMovementInput (Math|Vector|MakeVector 0.0 0.0 (Variables|Default|GetVerticalVelocity)) 1.0 false)))

(event Input|KeyboardEvents|R
  (params (Key :type Key%20Structure :default "None"))
  ;[1 1 1] Manually toggle enrage state
  (:Pressed
    (CallFunction|ServerToggleEnrage)))

(event Input|KeyboardEvents|V
  (params (Key :type Key%20Structure :default "None"))
  (:Pressed
    (CallFunction|ToggleHUD)))

(event Input|KeyboardEvents|Add
  (params (Key :type Key%20Structure :default "None"))
  (:Pressed
    (CallFunction|UpdateNumNPCs (Variables|Default|GetNPCDelta))))

(event Input|KeyboardEvents|Subtract
  (params (Key :type Key%20Structure :default "None"))
  (:Pressed
    (CallFunction|UpdateNumNPCs (* (Variables|Default|GetNPCDelta) -1))))

(event Input|KeyboardEvents|Z
  (params (Key :type Key%20Structure :default "None"))
  (:Pressed
    (CallFunction|StartCapture)
    (CallFunction|CaptureServer)))

(event Input|KeyboardEvents|SpaceBar
  (params (Key :type Key%20Structure :default "None"))
  ;[1 1 1] Spectator Controls, Space / Ctrl to go up / down
  (:Pressed
    (if (Variables|Default|GetIsSpectating)
      (Variables|Default|SetVerticalVelocity (Variables|/Script/Engine.CharacterMovementComponent|GetJumpZVelocity (Variables|Character|GetCharacterMovement)))))
  (:Released
    (Variables|Default|SetVerticalVelocity 0.0)))

(event Input|KeyboardEvents|LeftCtrl
  (params (Key :type Key%20Structure :default "None"))
  ;[1 1 1] Spectator Controls, Space / Ctrl to go up / down
  (:Pressed
    (if (Variables|Default|GetIsSpectating)
      (Variables|Default|SetVerticalVelocity (* (Variables|/Script/Engine.CharacterMovementComponent|GetJumpZVelocity (Variables|Character|GetCharacterMovement)) -1.0))))
  (:Released
    (Variables|Default|SetVerticalVelocity 0.0)))

(event Input|KeyboardEvents|K
  (params (Key :type Key%20Structure :default "None"))
  ;[1 1 1] Toggle spectator mode
  (:Pressed
    (CallFunction|ServerToggleSpectating)))

(fn ConstructionScript
  (|CallParentFunction))

(fn OnRepIsSpectating
  (Pawn|Components|CharacterMovement|SetMovementMode (Variables|Character|GetCharacterMovement) (select (Variables|Default|GetIsSpectating) "MOVE_Flying" "MOVE_Walking") 0)
  (Collision|SetActorEnableCollision (not (Variables|Default|GetIsSpectating)))
  (Rendering|SetActorHiddenInGame (Variables|Default|GetIsSpectating))
  (Variables|/Script/Engine.SpringArmComponent|SetbDoCollisionTest (Variables|Default|GetCameraBoom) (not (Variables|Default|GetIsSpectating))))

(fn CreateHUD
  (Networking|SwitchHasAuthority
    (:Remote
      (bind _returnvalue (UserInterface|CreateWidget "/Game/OffloadingBenchmark/UI_HUD.UI_HUD_C"))
      (bind _output_get (Variables|Default|SetHUD _returnvalue))
      (UserInterface|Viewport|AddtoViewport _returnvalue 0))))

(fn RemoveHUD
  (Networking|SwitchHasAuthority
    (:Remote
      (Widget|RemovefromParent (Variables|Default|GetHUD))
      (Variables|Default|SetHUD 0))))

(fn ToggleHUD
  (Variables|Default|GetHUD
    (:then
      (CallFunction|RemoveHUD))
    (:else
      (CallFunction|CreateHUD))))

(fn StartCapture
  (Development|ExecuteConsoleCommand "Stat StartFile" 0)
  (Utilities|Time|SetTimerbyEvent (EventDispatchers|CreateEvent :!event StopCapture) 1e+01))

(fn StopCapture
  (Development|ExecuteConsoleCommand "Stat StopFile" 0))