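; AI controller for NPCs in the offloading benchmark that starts their behavior tree and seeds its blackboard on possession.
; It copies the pawn's Enraged flag, sets TargetA to a random reachable navigation point within a large radius and TargetB to the pawn's starting location.
; It then sets the IsSettingValues flag to true after writing those keys.
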(event EventPossess
  (params (PossessedPawn :type Pawn%20Object%20Reference))
  (bind _blackboard (Variables|Default|GetBlackboard))
  (AI|RunBehaviorTree "/Game/OffloadingBenchmark/OffloadingBenchmark_NPCBehaviorTree.OffloadingBenchmark_NPCBehaviorTree")
  (AI|Components|Blackboard|SetValueasBool _blackboard (Utilities|Name|MakeLiteralName "Enraged") (Variables|/Game/OffloadingBenchmark/OffloadingBenchmark_CharacterBase_BP.OffloadingBenchmark_CharacterBase_BP_C|GetEnraged (.AsOffloading%20Benchmark%20Character%20Base%20BP (Utilities|Casting|CastToOffloadingBenchmark_CharacterBase_BP PossessedPawn))))
  (AI|Components|Blackboard|SetValueasVector _blackboard (Utilities|Name|MakeLiteralName "TargetA") (.RandomLocation (AI|Navigation|GetRandomReachablePointinRadius (Transformation|GetActorLocation (Pawn|GetControlledPawn)) 1e+04 0 0)))
  (AI|Components|Blackboard|SetValueasVector _blackboard (Utilities|Name|MakeLiteralName "TargetB") (Transformation|GetActorLocation (Pawn|GetControlledPawn)))
  (AI|Components|Blackboard|SetValueasBool _blackboard (Utilities|Name|MakeLiteralName "IsSettingValues") true))

(fn ConstructionScript)