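; Food pickup for the offloading benchmark that non-enraged benchmark characters eat to gain score.
; Overlap is handled only on the authority, which sets Eaten, awards score and starts a delayed respawn.
; The Eaten rep-notify hides the food, disables collision and moves it below ground.
; Respawn spawns a fresh food actor at a random reachable point within RespawnDistance, then destroys this one.
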(event Custom|StartRespawn
  (bind _returnvalue (Transformation|GetActorLocation))
  (Utilities|FlowControl|Delay (Variables|Default|GetSpawnInterval))
  (Utilities|FlowControl|DoOnce false
    (:Completed
      (Game|SpawnActorfromClass "OffloadingBenchmark_Food_BP_C" (Math|Transform|MakeTransform (.RandomLocation (AI|Navigation|GetRandomReachablePointinRadius (Math|Vector|MakeVector (.x _returnvalue) (.y _returnvalue) 0.0) (Variables|Default|GetRespawnDistance) 0 0)) "0, 0, 0" "1,1,1") "Undefined" 0 false 0)
      (Utilities|FlowControl|Delay 0.2)
      (Actor|DestroyActor))))

(event Collision|EventActorBeginOverlap
  (params (OtherActor :type Actor%20Object%20Reference))
  (Networking|SwitchHasAuthority
    (:Authority
      (bind _asoffloading_benchmark_character_base_bp (Utilities|Casting|CastToOffloadingBenchmark_CharacterBase_BP OtherActor))
      (if (not (Variables|/Game/OffloadingBenchmark/OffloadingBenchmark_CharacterBase_BP.OffloadingBenchmark_CharacterBase_BP_C|GetEnraged _asoffloading_benchmark_character_base_bp))
        (if (not (Variables|Default|GetEaten))
          (Variables|Default|SetEaten true)
          (Default|AddScore _asoffloading_benchmark_character_base_bp true)
          (CallFunction|StartRespawn))))))

(fn ConstructionScript
  (CallFunction|UpdateEaten))

(fn OnRepEaten
  (CallFunction|UpdateEaten))

(fn UpdateEaten
  (bind _returnvalue (Transformation|GetActorLocation))
  (Rendering|SetActorHiddenInGame (Variables|Default|GetEaten))
  (Collision|SetActorEnableCollision (not (Variables|Default|GetEaten)))
  (Transformation|SetActorLocation (Math|Vector|MakeVector (.x _returnvalue) (.y _returnvalue) (select (Variables|Default|GetEaten) -5e+02 0.0)) false false))