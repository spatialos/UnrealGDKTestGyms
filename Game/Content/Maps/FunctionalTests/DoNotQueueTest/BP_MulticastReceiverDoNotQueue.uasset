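; Receiver actor for a DoNotQueue functional test, printing through PrintStringSpatial when it gains server authority and when it is passed object references.
; MulticastPrintTreeName casts to StaticMeshActor and prints the mesh component's name whether or not the cast succeeds.
; PrintObjectName prints that name only if the reference casts to TestTreeRef.
; An "Unresolved Parameter" print is left unconnected.
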(event Custom|MulticastPrintTreeName
  (params (ObjectRef :type Actor%20Object%20Reference))
  (bind _asstatic_mesh_actor (Utilities|Casting|CastToStaticMeshActor ObjectRef)
    (:then
      _)
    (:CastFailed
      _))
  (Class|SpatialStatics|PrintStringSpatial (Utilities|GetDisplayName (Variables|/Script/Engine.StaticMeshActor|GetStaticMeshComponent _asstatic_mesh_actor))))

(event Custom|Print%20Object%20Name
  (params (ObjectRef :type Actor%20Object%20Reference))
  (bind _astest_tree_ref (Utilities|Casting|CastToTestTreeRef ObjectRef))
  (Class|SpatialStatics|PrintStringSpatial (Utilities|GetDisplayName (Variables|/Script/Engine.StaticMeshActor|GetStaticMeshComponent _astest_tree_ref))))

(event EventAuthorityGained
  (Class|SpatialStatics|PrintStringSpatial "Receiver Server Auth Gained"))

(fn ConstructionScript)