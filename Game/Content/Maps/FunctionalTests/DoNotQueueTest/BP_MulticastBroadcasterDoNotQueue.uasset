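; BP_MulticastBroadcasterDoNotQueue is the broadcaster in the DoNotQueue functional test, which contrasts queued and unqueued multicast events that carry an object reference.
; Both broadcast events log which variant executed, then find every BP_MulticastReceiverDoNotQueue.
; Each receiver with local authority is told to print the name of the passed MeshRef.
; Gaining authority only logs a message through Spatial print.
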(event Custom|Broadcast%20Reference%20to%20Cause%20Fails%20On%20Workers
  (params (MeshRef :type Test%20Tree%20Ref%20Object%20Reference))
  (Class|SpatialStatics|PrintStringSpatial "We executed the queued multicast")
  (bind _outactors (Actor|GetAllActorsOfClass "/Game/Maps/FunctionalTests/DoNotQueueTest/BP_MulticastReceiverDoNotQueue.BP_MulticastReceiverDoNotQueue_C"))
  (for _array_element _outactors
    (if (Ability|HasAuthority _array_element)
      (Default|PrintObjectName _array_element MeshRef))))

(event Custom|Broadcast%20References%20Not%20Queued
  (params (MeshRef :type Test%20Tree%20Ref%20Object%20Reference))
  (Class|SpatialStatics|PrintStringSpatial "We executed the unqueued multicast")
  (bind _outactors (Actor|GetAllActorsOfClass "/Game/Maps/FunctionalTests/DoNotQueueTest/BP_MulticastReceiverDoNotQueue.BP_MulticastReceiverDoNotQueue_C"))
  (for _array_element _outactors
    (if (Ability|HasAuthority _array_element)
      (Default|PrintObjectName _array_element MeshRef))))

(event EventBeginPlay)

(event EventAuthorityGained
  (Class|SpatialStatics|PrintStringSpatial "Broadcaster Auth Gained"))

(fn ConstructionScript)